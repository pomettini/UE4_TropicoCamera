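; BP_CameraController turns input axes into pan, yaw rotation and height-based zoom for player pawn 0, likely serving as the camera.
; All four axis events share one SetWorldLocationAndRotation call on the pawn's root component, fed by helper functions for movement, rotation and zoom.
; Panning follows forward and right vectors skewed 45 degrees from the pawn's facing.
; Zoom shifts Z within height limits, and no input is scaled by delta time.
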(event Input|AxisEvents|InputAxisVerticalMovement
  (params (AxisValue :type Float%20%28single-precision%29))
  (bind _returnvalue (Game|Player|GetPlayerPawn 0))
  (Transformation|SetWorldLocationAndRotation (Variables|/Script/Engine.Actor|GetRootComponent _returnvalue) (Utilities|HandleZoom (stale Input|AxisEvents|InputAxisWheelMovement AxisValue) (Utilities|HandleMovement (Utilities|LocalForwardVector _returnvalue) AxisValue (Utilities|LocalRightVector _returnvalue) (stale Input|AxisEvents|InputAxisHorizontalMovement AxisValue) (Transformation|GetActorLocation _returnvalue))) (Utilities|HandleRotation (Transformation|GetActorRotation _returnvalue) (stale Input|AxisEvents|InputAxisLateralMovement AxisValue)) false false))

(event Input|AxisEvents|InputAxisHorizontalMovement
  (params (AxisValue :type Float%20%28single-precision%29))
  (bind _returnvalue (Game|Player|GetPlayerPawn 0))
  (Transformation|SetWorldLocationAndRotation (Variables|/Script/Engine.Actor|GetRootComponent _returnvalue) (Utilities|HandleZoom (stale Input|AxisEvents|InputAxisWheelMovement AxisValue) (Utilities|HandleMovement (Utilities|LocalForwardVector _returnvalue) (stale Input|AxisEvents|InputAxisVerticalMovement AxisValue) (Utilities|LocalRightVector _returnvalue) AxisValue (Transformation|GetActorLocation _returnvalue))) (Utilities|HandleRotation (Transformation|GetActorRotation _returnvalue) (stale Input|AxisEvents|InputAxisLateralMovement AxisValue)) false false))

(event Input|AxisEvents|InputAxisWheelMovement
  (params (AxisValue :type Float%20%28single-precision%29))
  (bind _returnvalue (Game|Player|GetPlayerPawn 0))
  (Transformation|SetWorldLocationAndRotation (Variables|/Script/Engine.Actor|GetRootComponent _returnvalue) (Utilities|HandleZoom AxisValue (Utilities|HandleMovement (Utilities|LocalForwardVector _returnvalue) (stale Input|AxisEvents|InputAxisVerticalMovement AxisValue) (Utilities|LocalRightVector _returnvalue) (stale Input|AxisEvents|InputAxisHorizontalMovement AxisValue) (Transformation|GetActorLocation _returnvalue))) (Utilities|HandleRotation (Transformation|GetActorRotation _returnvalue) (stale Input|AxisEvents|InputAxisLateralMovement AxisValue)) false false))

(event Input|AxisEvents|InputAxisLateralMovement
  (params (AxisValue :type Float%20%28single-precision%29))
  (bind _returnvalue (Game|Player|GetPlayerPawn 0))
  (Transformation|SetWorldLocationAndRotation (Variables|/Script/Engine.Actor|GetRootComponent _returnvalue) (Utilities|HandleZoom (stale Input|AxisEvents|InputAxisWheelMovement AxisValue) (Utilities|HandleMovement (Utilities|LocalForwardVector _returnvalue) (stale Input|AxisEvents|InputAxisVerticalMovement AxisValue) (Utilities|LocalRightVector _returnvalue) (stale Input|AxisEvents|InputAxisHorizontalMovement AxisValue) (Transformation|GetActorLocation _returnvalue))) (Utilities|HandleRotation (Transformation|GetActorRotation _returnvalue) AxisValue) false false))

(fn ConstructionScript)